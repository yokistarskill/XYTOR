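; Player controller for top-down style control, moving the player pawn along world axes while it faces the mouse cursor.
; MoveX and MoveY axis inputs feed movement input on world X and Y, independent of facing.
; Each tick, the cursor is deprojected into a long Visibility trace, and the pawn snaps to look at the hit point, flattened to its own height.
; The trace result is used without checking for a hit.
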(event `InputAxis|MoveX`
  (params (AxisValue :type "Float (single-precision)"))
  (`Pawn.AddMovementInput` (`GameplayStatics.GetPlayerPawn` 0) (1.0 0.0 0.0) AxisValue false))

(event `InputAxis|MoveY`
  (params (AxisValue :type "Float (single-precision)"))
  (`Pawn.AddMovementInput` (`GameplayStatics.GetPlayerPawn` 0) (0.0 1.0 0.0) AxisValue false))

(event `self.ReceiveTick`
  (params (DeltaSeconds :type "Float (single-precision)"))
  (bind (_worldlocation _worlddirection _returnvalue) (`self.DeprojectMousePositionToWorld`))
  (bind _returnvalue_2 (`self.K2_GetActorLocation` (`GameplayStatics.GetPlayerPawn` 0)))
  (if _returnvalue
    (bind _outhit (`KismetSystemLibrary.LineTraceSingle` _worldlocation (+ _worldlocation (* _worlddirection 50000.0)) "TraceTypeQuery1"))
    (`self.K2_SetActorRotation` (`GameplayStatics.GetPlayerPawn` 0) (`KismetMathLibrary.FindLookAtRotation` _returnvalue_2 (`KismetMathLibrary.MakeVector` (.x (`.Location` (`GameplayStatics.BreakHitResult` _outhit))) (.y (`.Location` (`GameplayStatics.BreakHitResult` _outhit))) (.z _returnvalue_2))) false)))

(fn `UserConstructionScript`)