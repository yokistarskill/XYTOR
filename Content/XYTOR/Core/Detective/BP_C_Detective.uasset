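; BP_C_Detective is the Detective Blueprint, which uses an EvidenceFinder component to report evidence overlaps to its controller.
; It enables overlap events on EvidenceFinder at BeginPlay, then passes every overlapping actor to PC_Detective without filtering.
; The calls run opposite to their names: overlap begin calls UnDetectEvidence and overlap end calls DetectEvidence.
; Nothing happens when the controller is not a PC_Detective.
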(event `self.ReceiveBeginPlay`
  (`parent.ReceiveBeginPlay`)
  (set `PrimitiveComponent.bGenerateOverlapEvents` true (`self.EvidenceFinder`)))

(event `self.EvidenceFinder.OnComponentBeginOverlap`
  (params (OverlappedComponent :type "PrimitiveComponent Object Reference") (OtherActor :type "Actor Object Reference") (OtherComp :type "PrimitiveComponent Object Reference") (OtherBodyIndex :type Integer) (bFromSweep :type Boolean) (SweepResult :type "HitResult Structure (by ref)"))
  (bind _aspc_detective (cast `PC_Detective` (`self.GetController`)))
  (`PC_Detective.UnDetectEvidence` _aspc_detective OtherActor))

(event `self.EvidenceFinder.OnComponentEndOverlap`
  (params (OverlappedComponent :type "PrimitiveComponent Object Reference") (OtherActor :type "Actor Object Reference") (OtherComp :type "PrimitiveComponent Object Reference") (OtherBodyIndex :type Integer))
  (bind _aspc_detective (cast `PC_Detective` (`self.GetController`)))
  (`PC_Detective.DetectEvidence` _aspc_detective OtherActor))

(fn `UserConstructionScript`
  (`parent.UserConstructionScript`))